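; Player controller that streams procedural voxel terrain around the player by spawning and destroying ProceduralChunck actors.
; BeginPlay derives chunk size, picks a random seed shared by all chunks and spawns the initial set.
; Tick detects changes in the pawn's grid index, computed from half the chunk size, then removes and adds chunks.
; AddChunk scans a 5x5 neighborhood filtered by CheckRadius, tracking chunks in parallel coordinate and actor arrays.
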(event `self.ReceiveBeginPlay`
  (`self.initialize`)
  (`self.AddChunk`))

(event `self.ReceiveTick`
  (params (DeltaSeconds :type "Float (single-precision)"))
  (bind _waschanged (`self.UpdatePosition`))
  (if _waschanged
    (`self.removeChunck`)
    (`self.AddChunk`)))

(fn `AddChunk`
  (bind _chunkcords (`self.ChunkCords`))
  (bind _returnvalue (`KismetMathLibrary.Conv_IntToDouble` (`self.chunck Size`)))
  (bind _returnvalue_2 (`KismetMathLibrary.Conv_IntToDouble` (`self.chunck Size Half`)))
  (for _index (range -2 3)
    (for _index_2 (range -2 3)
      (bind _returnvalue_3 (+ _index (`self.chunck X`)))
      (bind _returnvalue_4 (* _returnvalue_3 _returnvalue))
      (bind _returnvalue_5 (+ _index_2 (`self.chunck Y`)))
      (bind _returnvalue_6 (* _returnvalue_5 _returnvalue))
      (if (`self.checkRadius` (+ _returnvalue_4 _returnvalue_2) (+ _returnvalue_6 _returnvalue_2))
        (bind _returnvalue_7 (`KismetMathLibrary.Conv_IntToDouble` _returnvalue_3))
        (bind _returnvalue_8 (`KismetMathLibrary.Conv_IntToDouble` _returnvalue_5))
        (if (not (`KismetArrayLibrary.Array_Contains` _chunkcords (`KismetMathLibrary.MakeVector2D` _returnvalue_7 _returnvalue_8)))
          (`KismetArrayLibrary.Array_Add` _chunkcords (`KismetMathLibrary.MakeVector2D` _returnvalue_7 _returnvalue_8))
          (bind _returnvalue_9 (`|SpawnActorFromClass` "/Game/Blueprints/ProceduralElements/ProceduralChunck.ProceduralChunck_C" (`KismetMathLibrary.Conv_VectorToTransform` (`KismetMathLibrary.MakeVector` _returnvalue_4 _returnvalue_6)) "Undefined" "OverrideRootScale" null (`self.lacunarity`) 3 0.6 (`self.seed`) (`self.voxelSize`) (`self.maxAltitude`) (+ (`self.chunckLineElements`) 2) _returnvalue_3 _returnvalue_5 null))
          (`KismetArrayLibrary.Array_Add` (`self.chuncks`) _returnvalue_9))))))

(fn `initialize`
  (bind _output_get (set `self.chunck Size` (* (`self.chunckLineElements`) (`self.voxelSize`))))
  (set `self.chunck Size Half` (/ _output_get 2))
  (set `self.seed` (`KismetMathLibrary.RandomInteger` 100000))
  (return))

(fn `removeChunck`
  (bind _chunck_size (`self.chunck Size`))
  (bind _chuncks (`self.chuncks`))
  (bind _returnvalue (`KismetMathLibrary.Conv_IntToDouble` (`self.chunck Size Half`)))
  (for (_array_element _array_index) (`self.ChunkCords`)
    (bind (_x _y) (`KismetMathLibrary.BreakVector2D` _array_element))
    (if (not (`self.checkRadius` (+ _returnvalue (* _chunck_size _x)) (+ _returnvalue (* _chunck_size _y))))
      (`self.K2_DestroyActor` (`|GetArrayItem` _chuncks _array_index))
      (`KismetArrayLibrary.Array_Remove` (`self.ChunkCords`) _array_index)
      (`KismetArrayLibrary.Array_Remove` _chuncks _array_index))))

(fn `UpdatePosition`
  (returns (wasChanged :type Boolean))
  (bind _returnvalue (`KismetMathLibrary.Conv_IntToDouble` (`self.chunck Size Half`)))
  (bind _output_get (set `self.characterPosition` (`self.K2_GetActorLocation` (`GameplayStatics.GetPlayerPawn` 0))))
  (bind _returnvalue_2 (`KismetMathLibrary.FFloor` (/ (.x _output_get) _returnvalue)))
  (bind _returnvalue_3 (`KismetMathLibrary.FFloor` (/ (.y _output_get) _returnvalue)))
  (if (or (!= (`self.chunck X`) _returnvalue_2) (!= (`self.chunck Y`) _returnvalue_3))
    (set `self.chunck X` _returnvalue_2)
    (set `self.chunck Y` _returnvalue_3)
    (return true)
    (else
      (return false))))

(fn `UserConstructionScript`)